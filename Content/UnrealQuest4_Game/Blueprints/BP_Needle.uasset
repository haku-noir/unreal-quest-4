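; BP_Needle is a hazard actor that damages the player on overlap and can be destroyed by projectiles.
; A BP_Projectile overlap plays an explosion sound, sets a destroyed flag that blocks further overlap responses, and removes the needle after a short delay.
; SpawnForceField spawns, triggers and immediately destroys a temporary FS_MasterField for a radial force, but its call in the event graph is disconnected and never runs.
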(event EventBeginPlay)

(event Collision|EventActorBeginOverlap
  (params (OtherActor :type Actor%20Object%20Reference))
  (if (not (Variables|Default|GetisDestroied))
    (Utilities|Casting|CastToBP_Projectile OtherActor
      (:then
        (Audio|PlaySoundatLocation "/Game/UnrealQuest4_Game/Audio/WAV_Explosion_Cue.WAV_Explosion_Cue" (Transformation|GetActorLocation OtherActor) "0, 0, 0" 1.0 1.0 0.0 0 0 0 0)
        (Variables|Default|SetisDestroied true)
        (Utilities|FlowControl|Delay 1.0)
        (Actor|DestroyActor))
      (:CastFailed
        (bind _asbp_uq4player (Utilities|Casting|CastToBP_UQ4Player OtherActor))
        (Game|Damage|ApplyDamage _asbp_uq4player 1.0 0 0)))))

(fn ConstructionScript)

(fn SpawnForceField
  (params (SpawnTransform :type Transform))
  (bind _returnvalue (Game|SpawnActorfromClass "/Engine/EditorResources/FieldNodes/FS_MasterField.FS_MasterField_C" SpawnTransform "Undefined" "MultiplyWithRoot" 0 0))
  (Components|Sphere|SetSphereRadius (Variables|/Engine/EditorResources/FieldNodes/FS_MasterField.FS_MasterField_C|GetSphereVolumeCol _returnvalue) 25.0 true)
  (Variables|/Engine/EditorResources/FieldNodes/FS_MasterField.FS_MasterField_C|SetRadial%20Magnitude _returnvalue 5e+03)
  (Default|CETrigger _returnvalue)
  (Actor|DestroyActor _returnvalue))