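; BP_MovingTarget is a target actor that moves by a MovingVector offset every tick until a projectile hits it.
; On its first overlap with a BP_Projectile, it spawns a BP_Target at its location and destroys itself.
; A SpawnForceField function, not called within this Blueprint, spawns a short-lived FS_MasterField to trigger a radial force burst.
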(event EventBeginPlay)

(event EventTick
  (params (DeltaSeconds :type Float%20%28single-precision%29))
  (Transformation|AddActorWorldOffset (Variables|Default|GetMoving%20Vector)))

(event Collision|EventActorBeginOverlap
  (params (OtherActor :type Actor%20Object%20Reference))
  (if (not (Variables|Default|GetisDestroied))
    (Utilities|Casting|CastToBP_Projectile OtherActor)
    (Game|SpawnActorfromClass "/Game/UnrealQuest4_Game/Blueprints/BP_Target.BP_Target_C" (Math|Conversions|ToTransform(Vector) (Transformation|GetActorLocation self)) "Undefined" "MultiplyWithRoot" 0 0)
    (Variables|Default|SetisDestroied true)
    (Actor|DestroyActor)))

(fn ConstructionScript)

(fn SpawnForceField
  (params (SpawnTransform :type Transform))
  (bind _returnvalue (Game|SpawnActorfromClass "/Engine/EditorResources/FieldNodes/FS_MasterField.FS_MasterField_C" SpawnTransform "Undefined" "MultiplyWithRoot" 0 0))
  (Components|Sphere|SetSphereRadius (Variables|/Engine/EditorResources/FieldNodes/FS_MasterField.FS_MasterField_C|GetSphereVolumeCol _returnvalue) 25.0 true)
  (Variables|/Engine/EditorResources/FieldNodes/FS_MasterField.FS_MasterField_C|SetRadial%20Magnitude _returnvalue 5e+03)
  (Default|CETrigger _returnvalue)
  (Actor|DestroyActor _returnvalue))