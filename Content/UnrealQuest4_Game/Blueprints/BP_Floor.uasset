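; BP_Floor is a floor actor that reacts to being hit by a BP_Projectile with an explosion and a burst of physics force.
; The first projectile overlap plays the explosion sound, sets a one-shot flag, spawns a force field and destroys the floor after a short delay.
; SpawnForceField creates a temporary FS_MasterField at the floor's location, sets its radius and radial magnitude, triggers it, then immediately destroys it.
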(event EventBeginPlay)

(event Collision|EventActorBeginOverlap
  (params (OtherActor :type Actor%20Object%20Reference))
  (if (not (Variables|Default|GetisDestroied))
    (Utilities|Casting|CastToBP_Projectile OtherActor)
    (Audio|PlaySoundatLocation "/Game/UnrealQuest4_Game/Audio/WAV_Explosion_Cue.WAV_Explosion_Cue" (Transformation|GetActorLocation OtherActor) "0, 0, 0" 1.0 1.0 0.0 0 0 0 0)
    (Variables|Default|SetisDestroied true)
    (CallFunction|SpawnForceField (Math|Conversions|ToTransform(Vector) (Transformation|GetActorLocation self)))
    (Utilities|FlowControl|Delay 2.0)
    (Actor|DestroyActor)))

(fn ConstructionScript)

(fn SpawnForceField
  (params (SpawnTransform :type Transform))
  (bind _returnvalue (Game|SpawnActorfromClass "/Engine/EditorResources/FieldNodes/FS_MasterField.FS_MasterField_C" SpawnTransform "Undefined" "MultiplyWithRoot" 0 0))
  (Components|Sphere|SetSphereRadius (Variables|/Engine/EditorResources/FieldNodes/FS_MasterField.FS_MasterField_C|GetSphereVolumeCol _returnvalue) 1e+02 true)
  (Variables|/Engine/EditorResources/FieldNodes/FS_MasterField.FS_MasterField_C|SetRadial%20Magnitude _returnvalue 5e+04)
  (Default|CETrigger _returnvalue)
  (Actor|DestroyActor _returnvalue))