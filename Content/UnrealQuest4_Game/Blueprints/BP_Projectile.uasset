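; BP_Projectile is a projectile that sets off a radial force field when it overlaps another actor.
; It plays a spawn sound on BeginPlay and destroys itself on Hit.
; Each overlap spawns a short-lived FS_MasterField at the projectile's transform, sets its sphere radius and radial magnitude, fires CETrigger, then destroys the field immediately.
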(event EventBeginPlay
  (Audio|PlaySoundatLocation "/Game/UnrealQuest4_Game/Audio/WAV_SpawnProjectile_Cue.WAV_SpawnProjectile_Cue" (Transformation|GetActorLocation) "0, 0, 0" 1.0 1.0 0.0 0 0 0 0))

(event Collision|EventActorBeginOverlap
  (params (OtherActor :type Actor%20Object%20Reference))
  (CallFunction|SpawnForceField (Transformation|GetActorTransform)))

(event EventTick
  (params (DeltaSeconds :type Float%20%28single-precision%29)))

(event Collision|EventHit
  (params (MyComp :type Primitive%20Component%20Object%20Reference) (Other :type Actor%20Object%20Reference) (OtherComp :type Primitive%20Component%20Object%20Reference) (bSelfMoved :type Boolean) (HitLocation :type Vector :default "0, 0, 0") (HitNormal :type Vector :default "0, 0, 0") (NormalImpulse :type Vector :default "0, 0, 0") (Hit :type Hit%20Result%20Structure%20%28by%20ref%29))
  (Actor|DestroyActor))

(fn ConstructionScript)

(fn SpawnForceField
  (params (SpawnTransform :type Transform))
  (bind _returnvalue (Game|SpawnActorfromClass "/Engine/EditorResources/FieldNodes/FS_MasterField.FS_MasterField_C" SpawnTransform "Undefined" "MultiplyWithRoot" 0 0))
  (Components|Sphere|SetSphereRadius (Variables|/Engine/EditorResources/FieldNodes/FS_MasterField.FS_MasterField_C|GetSphereVolumeCol _returnvalue) 5e+01 true)
  (Variables|/Engine/EditorResources/FieldNodes/FS_MasterField.FS_MasterField_C|SetRadial%20Magnitude _returnvalue 5e+03)
  (Default|CETrigger _returnvalue)
  (Actor|DestroyActor _returnvalue))