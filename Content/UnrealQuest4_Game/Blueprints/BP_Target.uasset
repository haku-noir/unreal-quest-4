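; BP_Target is a shootable target that awards the player score when hit by a BP_Projectile.
; On first overlap it calls an effect spawn and plays an explosion sound at the projectile, sets a destroyed flag, adds score to BP_UQ4Player, then destroys itself after a short delay.
; SpawnForceField fires a temporary FS_MasterField radial field for physics destruction, but its call is disconnected and never runs.
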(event EventBeginPlay)

(event Collision|EventActorBeginOverlap
  (params (OtherActor :type Actor%20Object%20Reference))
  (bind _returnvalue (Transformation|GetActorLocation OtherActor))
  (if (not (Variables|Default|GetisDestroied))
    (Utilities|Casting|CastToBP_Projectile OtherActor)
    (Niagara|SpawnSystematLocation 0 _returnvalue)
    (Audio|PlaySoundatLocation "/Game/UnrealQuest4_Game/Audio/WAV_Explosion_Cue.WAV_Explosion_Cue" _returnvalue "0, 0, 0" 1.0 1.0 0.0 0 0 0 0)
    (Variables|Default|SetisDestroied true)
    (bind _asbp_uq4player (Utilities|Casting|CastToBP_UQ4Player (Game|GetPlayerCharacter 0)))
    (Variables|/Game/UnrealQuest4_Game/ThirdPerson/Blueprints/BP_UQ4Player.BP_UQ4Player_C|SetScore _asbp_uq4player (+ (Variables|/Game/UnrealQuest4_Game/ThirdPerson/Blueprints/BP_UQ4Player.BP_UQ4Player_C|GetScore _asbp_uq4player) 1e+02))
    (Utilities|FlowControl|Delay 0.5)
    (Actor|DestroyActor)))

(fn ConstructionScript)

(fn SpawnForceField
  (params (SpawnTransform :type Transform))
  (bind _returnvalue (Game|SpawnActorfromClass "/Engine/EditorResources/FieldNodes/FS_MasterField.FS_MasterField_C" SpawnTransform "Undefined" "MultiplyWithRoot" 0 0))
  (Components|Sphere|SetSphereRadius (Variables|/Engine/EditorResources/FieldNodes/FS_MasterField.FS_MasterField_C|GetSphereVolumeCol _returnvalue) 25.0 true)
  (Variables|/Engine/EditorResources/FieldNodes/FS_MasterField.FS_MasterField_C|SetRadial%20Magnitude _returnvalue 5e+03)
  (Default|CETrigger _returnvalue)
  (Actor|DestroyActor _returnvalue))